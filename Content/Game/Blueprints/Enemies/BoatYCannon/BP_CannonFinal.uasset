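; Boat-mounted enemy cannon that snaps to BP_Boat's location each tick and targets a player inside its trigger.
; Trigger overlap runs a looping timer; OrientToPlayer yaws the base toward a predicted position via timeline, then launches a projectile by impulse.
; CannonPrediction leads the target by velocity and distance, using SuggestProjectileVelocityCustomArc for launch velocity.
; Pivot pitch, aim randomness and debug drawing are left disconnected.
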(event `self.ReceiveTick`
  (params (DeltaSeconds :type "Float (single-precision)"))
  (bind _returnvalue (`GameplayStatics.GetActorOfClass` "/Game/Game/Blueprints/Enemies/BoatYCannon/BP_Boat.BP_Boat_C"))
  (bind _returnvalue_2 (`self.GetTransform` _returnvalue))
  (`self.K2_SetActorLocation` (`KismetMathLibrary.MakeVector` (.x (.location _returnvalue_2)) (.y (.location _returnvalue_2)) (+ (.z (.location _returnvalue_2)) 20.0))))

(event `OrientToPlayer`
  (`TimelineComponent.SetPlayRate` (`self.OrientToThePlayer`) (/ 1.0 (`self.OrientationDuration`)))
  (`self.CacheRotationValues`)
  (bind (_direction _orient) (`Timeline|OrientToThePlayer` :!via `PlayFromStart`)
    (:`Update`
      (`SceneComponent.K2_SetWorldRotation` (`self.Base`) (`KismetMathLibrary.MakeRotator` 0.0 0.0 (.yaw (`KismetMathLibrary.RLerp` (`self.BaseRotation`) (`KismetMathLibrary.FindLookAtRotation` (`SceneComponent.K2_GetComponentLocation` (`self.Base`)) (`.Destino` (`self.CannonPrediction` (`self.PlayerCapsule`)))) _orient true))) false false))
    (:`Finished`
      (`self.CacheRotationValues`)
      (bind _returnvalue (`|SpawnActorFromClass` "/Game/Developers/diego/barco/BP_CannonProjectile.BP_CannonProjectile_C" (`SceneComponent.K2_GetComponentToWorld` (`self.Scene`)) "Undefined" "MultiplyWithRoot" null null))
      (`PrimitiveComponent.AddImpulse` (`/Game/Developers/diego/barco/BP_CannonProjectile.Sphere` _returnvalue) (* (`self.CannonPrediction` (`self.PlayerCapsule`)) (5.0 5.0 5.0)) "None" false))))

(event `self.Trigger.OnComponentBeginOverlap`
  (params (OverlappedComponent :type "PrimitiveComponent Object Reference") (OtherActor :type "Actor Object Reference") (OtherComp :type "PrimitiveComponent Object Reference") (OtherBodyIndex :type Integer) (bFromSweep :type Boolean) (SweepResult :type "HitResult Structure (by ref)"))
  (bind _asbp_player (cast `/Game/Game/Blueprints/Player/BP_Player` OtherActor))
  (set `self.PlayerCapsule` _asbp_player)
  (bind _returnvalue (`KismetSystemLibrary.K2_SetTimerDelegate` (`|CreateDelegate` :!event `OrientToPlayer`) 2.0 true))
  (set `self.OrientationTimer` _returnvalue))

(event `self.Trigger.OnComponentEndOverlap`
  (params (OverlappedComponent :type "PrimitiveComponent Object Reference") (OtherActor :type "Actor Object Reference") (OtherComp :type "PrimitiveComponent Object Reference") (OtherBodyIndex :type Integer))
  (cast `/Game/Game/Blueprints/Player/BP_Player` OtherActor)
  (`KismetSystemLibrary.K2_ClearAndInvalidateTimerHandle` (`self.OrientationTimer`)))

(fn `AddRandomnes`
  (params (Vector :type "Vector Structure") (Randomness :type "Float (double-precision)") (UseX :type Boolean :default true) (UseY :type Boolean :default true) (UseZ :type Boolean :default true))
  (returns (ReturnValue :type "Vector Structure"))
  (bind _x (.x Vector))
  (bind _y (.y Vector))
  (bind _z (.z Vector))
  (bind _returnvalue (* Randomness 0.0))
  (return (`KismetMathLibrary.MakeVector` (`KismetMathLibrary.SelectFloat` (+ _x (`KismetMathLibrary.RandomFloatInRange` _returnvalue Randomness)) _x UseX) (`KismetMathLibrary.SelectFloat` (+ _y (`KismetMathLibrary.RandomFloatInRange` _returnvalue Randomness)) _y UseY) (`KismetMathLibrary.SelectFloat` (+ _z (`KismetMathLibrary.RandomFloatInRange` _returnvalue Randomness)) _z UseZ))))

(fn `CacheRotationValues`
  (set `self.PivotRotation` (`SceneComponent.RelativeRotation` (`self.Pivot`)))
  (set `self.BaseRotation` (`SceneComponent.K2_GetComponentRotation` (`self.Base`))))

(fn `CannonPrediction`
  (params (character :type "Character Object Reference"))
  (returns (DesiredVelocity :type "Vector Structure") (Destino :type "Vector Structure"))
  (bind _returnvalue (+ (`self.TargetActorLocation`) (* (`self.TargetActorVelocity`) (/ (`KismetMathLibrary.Vector_Distance` (`self.TargetActorLocation`) (`self.K2_GetActorLocation`)) 1200.0))))
  (set `self.TargetActorVelocity` (`CharacterMovementComponent.GetLastUpdateVelocity` (`Character.CharacterMovement` character)))
  (set `self.TargetActorLocation` (`CharacterMovementComponent.GetLastUpdateLocation` (`Character.CharacterMovement` character)))
  (bind _outlaunchvelocity (`GameplayStatics.SuggestProjectileVelocity_CustomArc` (`SceneComponent.K2_GetComponentLocation` (`self.Scene`)) _returnvalue))
  (if true
    (return _outlaunchvelocity _returnvalue)))

(fn `UserConstructionScript`)