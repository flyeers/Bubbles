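; Player Blueprint that only implements a death reaction through the Dead event.
; Dead rolls the Mesh from its current rotation and moves the actor downward without sweep, in a single call with no timeline.
; Both lerps use an Alpha far above 1, so they extrapolate well past the intended-looking 90-degree roll and 100-unit drop instead of blending.
; BeginPlay, overlap, Tick and the construction script are empty.
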(event `Dead`
  (bind (_relativerotation_roll _relativerotation_pitch _relativerotation_yaw) (`KismetMathLibrary.BreakRotator` (`SceneComponent.RelativeRotation` (`self.Mesh`))))
  (`SceneComponent.K2_SetRelativeRotation` (`self.Mesh`) (`KismetMathLibrary.RLerp` (`SceneComponent.RelativeRotation` (`self.Mesh`)) (`KismetMathLibrary.MakeRotator` (+ _relativerotation_roll 90.0) _relativerotation_pitch _relativerotation_yaw) 15.0) false false)
  (`self.K2_SetActorLocation` (`KismetMathLibrary.VLerp` (`self.K2_GetActorLocation`) (- (`self.K2_GetActorLocation`) (0.0 0.0 100.0)) 15.0)))

(fn `UserConstructionScript`)