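; Shark enemy AI Blueprint that uses AI Perception to pick the player as a follow target.
; A macro filters stimuli for BP_PlayerD; a successful sensing clears the memory timer and writes the player to the Blackboard follow key.
; A timed forget function can clear that key, but LostTrackOfTarget, which starts its timer, is unwired, so the target is never forgotten.
; Debug prints mark perception updates and forgetting.
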(event `self.AIPerception.OnTargetPerceptionUpdated`
  (params (Actor :type "Actor Object Reference") (Stimulus :type "AIStimulus Structure"))
  (`KismetSystemLibrary.PrintString` "HE VISTO ALGO")
  (`self.ProcessTimuli` Actor Stimulus
    (:`FollowNewActor`
      (`self.FollowNewActor` Actor))))

(fn `FollowNewActor`
  (params (ObjectValue :type "Object Object Reference"))
  (`KismetSystemLibrary.K2_ClearAndInvalidateTimerHandle` (`self.MemoryDurationTimer`))
  (`BlackboardComponent.SetValueAsObject` (`AIBlueprintHelperLibrary.GetBlackboard` null) (`self.FollowTargetKey`) ObjectValue)
  (return))

(fn `Forget About Target`
  (`KismetSystemLibrary.PrintString` "OLVIDADO")
  (`BlackboardComponent.SetValueAsObject` (`AIBlueprintHelperLibrary.GetBlackboard` null) (`self.FollowTargetKey`) null))

(fn `LostTrackOfTarget`
  (locals (MemoryDuration :type "Float (double-precision)" :default 1.0))
  (bind _returnvalue (`KismetSystemLibrary.K2_SetTimer` null "ForgetAboutTarget" (`local.MemoryDuration`)))
  (set `self.MemoryDurationTimer` _returnvalue)
  (return))

(fn `UserConstructionScript`)