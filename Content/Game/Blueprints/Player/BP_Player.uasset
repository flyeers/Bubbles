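; BP_Player is the playable duck character, driven by Enhanced Input for turning and moving, shooting projectiles and turbo sprinting.
; A shared water resource gates shooting and sprinting, drains as they are used and refills on Tick while the duck is stationary.
; Each water change updates a water bar widget component.
; Movement input spawns randomly offset bubbles behind an arrow component, in bursts when sprinting and occasionally otherwise.
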(event `self.ReceiveBeginPlay`
  (bind _maxwater (`self.MaxWater`))
  ;[1 1 1] Set Input Mapping
  (bind _asplayer_controller (cast `PlayerController` (`self.GetController`)))
  (bind _returnvalue (pcsubsystem `EnhancedInputLocalPlayerSubsystem` _asplayer_controller))
  (`/Engine/EditorBlueprintResources/StandardMacros.IsValid` _returnvalue
    (:`Is Valid`
      (`EnhancedInputSubsystemInterface.AddMappingContext` _returnvalue "/Game/Game/Blueprints/Player/Input/Duck_InputMapping.Duck_InputMapping" 0 (struct))
      ;[1 1 1] Water Resource + UI
      (set `self.CurrentWater` (`self.MaxWater`))
      (bind _asbp_water_bar_widget (cast `/Game/Game/Blueprints/UI/BP_WaterBarWidget` (`WidgetComponent.GetUserWidgetObject` (`self.WaterBar`))))
      (bind _output_get (set `self.WaterBarWidget` _asbp_water_bar_widget))
      (set `/Game/Game/Blueprints/UI/BP_WaterBarWidget.MaxWater` _maxwater _output_get)
      (`/Game/Game/Blueprints/UI/BP_WaterBarWidget.SetWater` _output_get _maxwater))))

(event `self.ReceiveTick`
  (params (DeltaSeconds :type "Float (single-precision)"))
  ;[1 1 1] Add Water resource
  (if (== (`KismetMathLibrary.VSize` (`self.GetVelocity`)) 0.0)
    (`KismetSystemLibrary.Delay` 0.2)
    (if (< (`self.CurrentWater`) (`self.MaxWater`))
      (bind _output_get (set `self.CurrentWater` (+ (`self.CurrentWater`) (`self.AddIncrement`))))
      (`/Game/Game/Blueprints/UI/BP_WaterBarWidget.SetWater` (`self.WaterBarWidget`) _output_get))))

(event `EnhancedInput|/Game/Game/Blueprints/Player/Input/IA_Movement`
  (params (ActionValue :type "Vector2D Structure") (ElapsedSeconds :type "Float (double-precision)") (TriggeredSeconds :type "Float (double-precision)") (InputAction :type "InputAction Object Reference" :default "/Game/Game/Blueprints/Player/Input/IA_Movement.IA_Movement"))
  (bind (_returnvalue_location _returnvalue_rotation _returnvalue_scale) (`KismetMathLibrary.BreakTransform` (`SceneComponent.K2_GetComponentToWorld` (`self.Arrow2`))))
  (bind _returnvalue (+ _returnvalue_location (`KismetMathLibrary.RandomFloatInRange` -20.0 20.0)))
  ;[1 1 1] MOVEMENT
  (:`Triggered`
    (`SceneComponent.K2_AddLocalRotation` (`self.Duck`) (`KismetMathLibrary.MakeRotator` 0.0 0.0 (* ActionValue_X (`self.RotationSpeed`))) false false)
    (`self.AddMovementInput` (`SceneComponent.GetForwardVector` (`self.Arrow1`)) ActionValue_Y)
    ;[1 1 1] Bubble effect
    (if (`self.sprinting`)
      (if true
        (`|SpawnActorFromClass` "/Game/Game/Blueprints/Player/Bubble.Bubble_C" (`KismetMathLibrary.MakeTransform` _returnvalue) "Undefined" "MultiplyWithRoot" null null)
        (`|SpawnActorFromClass` "/Game/Game/Blueprints/Player/Bubble.Bubble_C" (`KismetMathLibrary.MakeTransform` _returnvalue) "Undefined" "MultiplyWithRoot" null null)
        (`|SpawnActorFromClass` "/Game/Game/Blueprints/Player/Bubble.Bubble_C" (`KismetMathLibrary.MakeTransform` _returnvalue _returnvalue_rotation _returnvalue_scale) "Undefined" "MultiplyWithRoot" null null)
        (`|SpawnActorFromClass` "/Game/Game/Blueprints/Player/Bubble.Bubble_C" (`KismetMathLibrary.MakeTransform` _returnvalue) "Undefined" "MultiplyWithRoot" null null :!label _label))
      (elif (== (`KismetMathLibrary.RandomIntegerInRange` 0 2) 1)
        (goto _label)))))

(event `EnhancedInput|/Game/Game/Blueprints/Player/Input/IA_Shoot`
  (params (ActionValue :type Boolean) (ElapsedSeconds :type "Float (double-precision)") (TriggeredSeconds :type "Float (double-precision)") (InputAction :type "InputAction Object Reference" :default "/Game/Game/Blueprints/Player/Input/IA_Shoot.IA_Shoot"))
  ;[1 1 1] Shoot
  (:`Triggered`
    (if (> (`self.CurrentWater`) 0.0)
      (`KismetSystemLibrary.Delay` 0.1)
      (`|SpawnActorFromClass` "/Game/Game/Blueprints/Player/BP_Projectile.BP_Projectile_C" (`SceneComponent.K2_GetComponentToWorld` (`self.Arrow1`)) "AlwaysSpawn" "MultiplyWithRoot" null null)
      ;[1 1 1] Substract water resource
      (bind _output_get (set `self.CurrentWater` (`KismetMathLibrary.FMax` (- (`self.CurrentWater`) (`self.SubstractIncrement`))) :!label _label_2))
      (`/Game/Game/Blueprints/UI/BP_WaterBarWidget.SetWater` (`self.WaterBarWidget`) _output_get))))

(event `EnhancedInput|/Game/Game/Blueprints/Player/Input/IA_Turbo`
  (params (ActionValue :type Boolean) (ElapsedSeconds :type "Float (double-precision)") (TriggeredSeconds :type "Float (double-precision)") (InputAction :type "InputAction Object Reference" :default "/Game/Game/Blueprints/Player/Input/IA_Turbo.IA_Turbo"))
  (bind _charactermovement (`self.CharacterMovement`))
  ;[1 1 1] Sprint
  (:`Triggered`
    (if (!= (`KismetMathLibrary.VSize` (`self.GetVelocity`)) 0.0)
      (if (> (`self.CurrentWater`) 0.0)
        (set `CharacterMovementComponent.MaxWalkSpeed` (`self.SprintSpeed`) _charactermovement)
        (set `self.sprinting` true)
        (goto _label_2)
        (else
          (set `CharacterMovementComponent.MaxWalkSpeed` 1500.0 _charactermovement :!label _label_3)
          (set `self.sprinting` false)))))
  (:`Completed`
    (goto _label_3)))

(fn `UserConstructionScript`)