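; BP_PatitoHijo is a duckling character that follows the player and registers itself with them on contact.
; On BeginPlay it caches BP_Player and sets its walk speed slightly above the player's.
; Tick, plus a delayed retry on success, issues AI MoveTo toward the player within a set distance band.
; A capsule hit calls the player's AddPatito through a DoOnce that resets only when the hit actor is not the player.
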(event `self.ReceiveBeginPlay`
  (`KismetSystemLibrary.PrintString` (`KismetStringLibrary.Conv_RotatorToString` (`self.K2_GetActorRotation`)))
  (bind _asbp_player (cast `/Game/Game/Blueprints/Player/BP_Player` (`GameplayStatics.GetPlayerCharacter` 0)))
  (bind _output_get (set `self.Player Ref` _asbp_player))
  (set `CharacterMovementComponent.MaxWalkSpeed` (+ (`CharacterMovementComponent.MaxWalkSpeed` (`Character.CharacterMovement` _output_get)) 200.0) (`self.CharacterMovement`)))

(event `self.ReceiveTick`
  (params (DeltaSeconds :type "Float (single-precision)"))
  (`self.Follow Player`))

(event `Follow Player`
  (bind _returnvalue (`self.GetDistanceTo` (`self.Player Ref`)))
  (if (and (>= _returnvalue 50.0) (<= _returnvalue 2000.0))
    (`|AIMoveTo` self (0.0 0.0 0.0) (`self.Player Ref`)
      (:`OnSuccess`
        (`KismetSystemLibrary.Delay` 0.2)
        (`self.Follow Player`)))))

(event `self.CapsuleComponent.OnComponentHit`
  (params (HitComponent :type "PrimitiveComponent Object Reference") (OtherActor :type "Actor Object Reference") (OtherComp :type "PrimitiveComponent Object Reference") (NormalImpulse :type "Vector Structure") (Hit :type "HitResult Structure (by ref)"))
  (`/Engine/EditorBlueprintResources/StandardMacros.DoOnce` false :!label _label
    (:`Completed`
      (bind _asbp_player (cast `/Game/Game/Blueprints/Player/BP_Player` OtherActor)
        (:`then`
          (`/Game/Game/Blueprints/Player/BP_Player.AddPatito` _asbp_player))
        (:`CastFailed`
          (goto _label :!via `Reset`))))))

(fn `UserConstructionScript`)