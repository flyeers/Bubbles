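; Enemy boat that perceives the player and sinks them when its box collider overlaps them.
; AI perception updates pass through the Stimulu macro, which filters for BP_Player: a sighting writes the blackboard target and cancels the memory timer.
; Losing the player starts a MemoryDuration timer meant to clear the target.
; That timer calls "ForgetAboutTarget", while the clearing function here is named ForgetTarget.
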(event `self.AIPerception.OnTargetPerceptionUpdated`
  (params (Actor :type "Actor Object Reference") (Stimulus :type "AIStimulus Structure"))
  (`self.Stimulu` Actor Stimulus
    (:`FollowNewActor`
      (`self.FollowNewActor` Actor))
    (:`LostTrackOfTarget`
      (`self.LostTrackOfTarget`))))

(event `self.Box.OnComponentBeginOverlap`
  (params (OverlappedComponent :type "PrimitiveComponent Object Reference") (OtherActor :type "Actor Object Reference") (OtherComp :type "PrimitiveComponent Object Reference") (OtherBodyIndex :type Integer) (bFromSweep :type Boolean) (SweepResult :type "HitResult Structure (by ref)"))
  (bind _asbp_player (cast `/Game/Game/Blueprints/Player/BP_Player` OtherActor))
  (`/Game/Game/Blueprints/Player/BP_Player.Sink` _asbp_player))

(fn `FollowNewActor`
  (params (ObjectValue :type "Object Object Reference"))
  (`KismetSystemLibrary.K2_ClearAndInvalidateTimerHandle` (`self.MemoryDurationTimer`))
  (`BlackboardComponent.SetValueAsObject` (`AIBlueprintHelperLibrary.GetBlackboard` null) (`self. Target key`) ObjectValue)
  (return))

(fn `ForgetTarget`
  (`KismetSystemLibrary.PrintString` "OLVIDADO")
  (`BlackboardComponent.SetValueAsObject` (`AIBlueprintHelperLibrary.GetBlackboard` null) (`self. Target key`) null))

(fn `LostTrackOfTarget`
  (locals (`Memory Duration` :type "Float (double-precision)"))
  (bind _returnvalue (`KismetSystemLibrary.K2_SetTimer` null "ForgetAboutTarget" (`local.Memory Duration`)))
  (set `self.MemoryDurationTimer` _returnvalue)
  (return))

(fn `UserConstructionScript`)